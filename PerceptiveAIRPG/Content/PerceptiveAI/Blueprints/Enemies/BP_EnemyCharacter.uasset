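; BP_EnemyCharacter is an enemy character that tracks its health and reports basic combat state.
; BeginPlay sets Health to MaxHealth, and query functions return current and maximum health, alive status and a false IsPlayer flag.
; GetAttackRange returns zero for both minimum and maximum range, and nothing in this graph changes Health after initialization.
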(event `self.ReceiveBeginPlay`
  (set `self.Health` (`self.MaxHealth`)))

(fn `GetAttackRange`
  (returns (MaxRange :type "Float (double-precision)") (MinRange :type "Float (double-precision)"))
  (return 0.0 0.0))

(fn `GetHealth`
  (returns (CurrentHealth :type "Float (double-precision)") (MaxHealth :type "Float (double-precision)"))
  (return (`self.Health`) (`self.MaxHealth`)))

(fn `IsAlive`
  (returns (bAlive :type Boolean))
  (return (> (`self.Health`) 0.0)))

(fn `IsPlayer`
  (returns (bPlayer :type Boolean))
  (return false))

(fn `UserConstructionScript`)